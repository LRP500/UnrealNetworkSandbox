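; Gameplay player controller that sets up the in-game leave-session UI and mouse-friendly input for the local player.
; On BeginPlay, only when locally controlled, it adds a WBP_LeaveSession widget to the viewport, then calls SetInputMode.
; SetInputMode targets player controller index 0 rather than self, showing the cursor, applying Game and UI input mode and printing a debug confirmation.
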(event `self.ReceiveBeginPlay`
  (if (`self.IsLocalController`)
    (`self.CreateUI`
      (:`Out`
        (`self.SetInputMode`)))))

(fn `UserConstructionScript`)
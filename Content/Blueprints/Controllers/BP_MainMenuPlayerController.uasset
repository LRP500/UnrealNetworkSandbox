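; BP_MainMenuPlayerController is the player controller for the main menu, which shows the menu interface to the local player.
; On BeginPlay, local controllers only call CreateUI to add a WBP_MainMenu widget to the viewport, then SetInputMode.
; SetInputMode shows the mouse cursor, switches input to UI only and prints a confirmation message on screen.
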(event `self.ReceiveBeginPlay`
  (if (`self.IsLocalController`)
    (`self.CreateUI`)
    (`self.SetInputMode`)))

(fn `UserConstructionScript`)